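; Observable actor that destroys itself once the player camera has kept it in view for a set time, using settings from Data.
; While its attach parent was recently rendered, Tick checks camera distance, then line-traces from offset points to the camera.
; Enough unblocked traces advance the observation timer.
; Too few reset it after a tolerance period, while leaving range resets it immediately.
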(event `self.ReceiveBeginPlay`
  ;[0.662 0.8102 1] PLAYING
  (set `self.OBSTime` (`/Game/OldTool/DataAsset/BD_ObservableData.OBSTime` (`self.Data`)))
  (set `self.Max View Distance` (`/Game/OldTool/DataAsset/BD_ObservableData.Max View Distance` (`self.Data`)))
  (set `self.Tolerance Threshold` (`/Game/OldTool/DataAsset/BD_ObservableData.Tolerance Threshold` (`self.Data`)))
  (set `self.Success Threshold` (`/Game/OldTool/DataAsset/BD_ObservableData.Success Threshold` (`self.Data`))))

(event `Counter Manager`
  ;[0.8097 1 0.5398] Counter Manager
  (if (>= (`self.Sucess Rate`) (- (`KismetArrayLibrary.Array_Length` (`/Game/OldTool/DataAsset/BD_ObservableData.Positions` (`self.Data`))) (`self.Success Threshold`)))
    (set `self.Counter` (+ (`self.Counter`) (`GameplayStatics.GetWorldDeltaSeconds`)))
    (set `self.Tolerance Counter` 0.0)
    (if (>= (`self.Counter`) (`self.OBSTime`))
      (`self.SetActorTickEnabled` false)
      (`self.K2_DestroyActor`))
    (else
      (set `self.Tolerance Counter` (+ (`self.Tolerance Counter`) (`GameplayStatics.GetWorldDeltaSeconds`)) :!label _label)
      (if (>= (`self.Tolerance Counter`) (`self.Tolerance Threshold`))
        (set `self.Counter` 0.0)))))

(event `LineTrace`
  ;[1 1 1] Check visibility
  (set `self.Sucess Rate` 0)
  (for _index (range (+ (`KismetArrayLibrary.Array_LastIndex` (`/Game/OldTool/DataAsset/BD_ObservableData.Positions` (`self.Data`))) 1))
    (bind (_outhit _returnvalue) (`KismetSystemLibrary.LineTraceSingleForObjects` :`Start` (+ (`|GetArrayItem` (`/Game/OldTool/DataAsset/BD_ObservableData.Positions` (`self.Data`)) _index) (`self.K2_GetActorLocation`)) :`End` (`PlayerCameraManager.GetCameraLocation` (`GameplayStatics.GetPlayerCameraManager` 0)) :`ObjectTypes` (`self.Object Types`) :`DrawTime` 3.0))
    (if (not _returnvalue)
      (`/Engine/EditorBlueprintResources/StandardMacros.IncrementInt` (`self.Sucess Rate`))))
  (`self.Counter Manager`))

(event `Inverse Count`
  ;[0.8097 1 0.5398] Counter Manager
  (goto _label))

(event `self.ReceiveTick`
  (params (DeltaSeconds :type "Float (single-precision)"))
  ;[1 0.6283 0.5684] THICK
  (if (`self.WasRecentlyRendered` (`self.GetAttachParentActor`) 1.0)
    (`self.Distance Check`)))

(event `Distance Check`
  ;[1 1 1] Distance Check
  (if (<= (* (`KismetMathLibrary.Vector_Distance` (`PlayerCameraManager.GetCameraLocation` (`GameplayStatics.GetPlayerCameraManager` 0)) (`self.K2_GetActorLocation`)) 0.01) (`self.Max View Distance`))
    (`self.LineTrace`)
    (else
      (set `self.Counter` 0.0)
      (`self.Inverse Count`))))

(fn `UserConstructionScript`)