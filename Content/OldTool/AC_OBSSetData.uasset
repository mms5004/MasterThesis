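; Actor component from the OldTool folder that exports its owner's observation point layout to a new data asset.
; CreateData finds the owner's scene component named "OBSPoints" and gathers the relative locations of all its descendants, each relative to its own parent.
; It passes them to a constructed EUBA_ObservationData object's CreateNewDataAsset, leaving the entity name as None.
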(event `Create Data`
  (for _array_element (`Actor.K2_GetComponentsByClass` (`self.GetOwner`) "/Script/Engine.SceneComponent")
    (if (== (`KismetSystemLibrary.GetObjectName` _array_element) "OBSPoints")
      (`|ExecutionSequence`
        (:`then_0`
          (break))
        (:`then_1`
          (bind _returnvalue (`|GenericCreateObject` "/Game/OldTool/EUBA_ObservationData.EUBA_ObservationData_C"))
          (bind _pos (`self.Get All Children Pos` _array_element))
          (`/Game/OldTool/BPI_ToolData.CreateNewDataAsset` _returnvalue "None" _pos))))))

(fn `Get All Children Pos`
  (params (Component :type "SceneComponent Object Reference"))
  (returns (Pos :type "Array of Vector Structure"))
  (locals (LocalPos :type "Array of Vector Structure"))
  (for _array_element (`SceneComponent.GetChildrenComponents` Component true)
    (`KismetArrayLibrary.Array_Add` (`local.LocalPos`) (`SceneComponent.RelativeLocation` _array_element)))
  (return (`local.LocalPos`)))