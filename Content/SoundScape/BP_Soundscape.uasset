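; BP_Soundscape is a trigger volume that switches Soundscape audio while something overlaps its Box.
; On BeginPlay it derives the palette collection name from its SoundscapeState gameplay tag.
; Begin overlap registers the PaletteCollection with the Soundscape subsystem, sets the state and prints an on-screen message; end overlap removes both.
; Overlaps are not filtered by actor or counted, so any exit clears the state.
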(event `self.ReceiveBeginPlay`
  (set `self.Palette Collection Name` (`BlueprintGameplayTagLibrary.GetTagName` (`self.Soundscape State`))))

(event `self.Box.OnComponentBeginOverlap`
  (params (OverlappedComponent :type "PrimitiveComponent Object Reference") (OtherActor :type "Actor Object Reference") (OtherComp :type "PrimitiveComponent Object Reference") (OtherBodyIndex :type Integer) (bFromSweep :type Boolean) (SweepResult :type "HitResult Structure (by ref)"))
  (bind _returnvalue (subsystem `SoundscapeSubsystem`))
  (`SoundscapeSubsystem.AddPaletteCollection` _returnvalue (`self.Palette Collection Name`) (`self.Palette Collection`))
  (`SoundscapeSubsystem.SetState` _returnvalue (`self.Soundscape State`))
  (`KismetSystemLibrary.PrintString` "Hello" true false))

(event `self.Box.OnComponentEndOverlap`
  (params (OverlappedComponent :type "PrimitiveComponent Object Reference") (OtherActor :type "Actor Object Reference") (OtherComp :type "PrimitiveComponent Object Reference") (OtherBodyIndex :type Integer))
  (bind _returnvalue (subsystem `SoundscapeSubsystem`))
  (`SoundscapeSubsystem.RemovePaletteCollection` _returnvalue (`self.Palette Collection Name`))
  (`SoundscapeSubsystem.ClearState` _returnvalue (`self.Soundscape State`)))

(fn `UserConstructionScript`)